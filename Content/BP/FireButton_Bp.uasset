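; FireButton_Bp is an interactable button tied to a workspace object's fire effect that advances the current task when used.
; On Interact, it checks that it is interactable and that the Fire04 component on WorkSpaceThing is active.
; It then disables further interaction, tells TaskManager to change task, and flags itself as deactivated.
; BeginPlay and construction only call the parent class.
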(event EventBeginPlay
  (|CallParentFunction))

(event Collision|EventActorBeginOverlap
  (params (OtherActor :type Actor%20Object%20Reference)))

(event EventTick
  (params (DeltaSeconds :type Float%20%28single-precision%29)))

(event EventInteract
  (if (Variables|Default|GetIsInteractable)
    (if (Components|Activation|IsActive (Variables|/Game/BP/WorkSpaceThing.WorkSpaceThing_C|GetFire_04 (Variables|Default|GetWorkSpaceThing)))
      (Variables|Default|SetIsInteractable false)
      (Default|ChangeTask (Variables|Default|GetTaskManager))
      (Variables|Default|SetIsDeactivated true))))

(fn ConstructionScript
  (|CallParentFunction))